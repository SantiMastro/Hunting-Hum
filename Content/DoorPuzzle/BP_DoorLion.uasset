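; BP_DoorLion is a puzzle door that swings open and closed through OpenDoor and CloseDoor events.
; OpenDoor plays a squeak sound and runs a timeline whose yaw value combines with the mesh's default world rotation.
; CloseDoor reverses that timeline without sound.
; The default rotation is cached only after a ten-second delay at BeginPlay.
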(event Custom|OpenDoor
  (Audio|PlaySoundatLocation "/Game/Audio/346211__inspectorj__door-squeak-normal-e.346211__inspectorj__door-squeak-normal-e" (Transformation|GetActorLocation) "0, 0, 0" 1.0 1.0 0.0 0 0 0 0)
  (bind _dooranim (Timeline|DoorTimeline Play)
    (:Update
      (Transformation|SetWorldRotation (Variables|Debug|GetStaticMeshComponent) (Math|Rotator|CombineRotators (Math|Rotator|MakeRotator 0.0 0.0 _dooranim) (Variables|Default|GetDefaultRotation)) false false))))

(event Custom|CloseDoor
  (bind _dooranim (Timeline|DoorTimeline Reverse)
    (:Update
      (Transformation|SetWorldRotation (Variables|Debug|GetStaticMeshComponent) (Math|Rotator|CombineRotators (Math|Rotator|MakeRotator 0.0 0.0 _dooranim) (Variables|Default|GetDefaultRotation)) false false))))

(event EventBeginPlay
  (Utilities|FlowControl|Delay 1e+01)
  (Variables|Default|SetDefaultRotation (Transformation|GetWorldRotation (Variables|Debug|GetStaticMeshComponent))))

(fn ConstructionScript)