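; Zombie enemy that detects the player by sight and sound, plays chase music and performs a headbutt attack.
; PawnSensing sets AI blackboard keys for seeing and hearing, with a looping timer clearing the sight key.
; Chase music starts once per sighting and fades on Tick after sight lapses.
; AttackPlayer plays a montage and immediately sphere-traces forward, applying damage and a jumpscare sound on a hit.
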(event OnSeePawn(PawnSensing)
  (params (Pawn :type Pawn%20Object%20Reference))
  (Utilities|FlowControl|Sequence
    (:then_0
      (Variables|Default|SetSee%20Enemy true)
      (if (Actor|ActorHasTag Pawn "Player")
        (AI|Components|Blackboard|SetValueasBool (AI|GetBlackboard (AI|GetAIController self)) (Utilities|Name|MakeLiteralName "seeingPlayer") true)
        (Utilities|FlowControl|DoOnce false
          (:Completed
            (Audio|Components|Audio|Play (Variables|Default|GetChaseMusic) 0.0)))))
    (:then_1
      (Utilities|FlowControl|RetriggerableDelay 0.6)
      (Variables|Default|SetSee%20Enemy false))))

(event OnAudioFinished(Audio)
  (Audio|Components|Audio|Play (Variables|Default|GetAudio) 0.0))

(event OnHearNoise(PawnSensing)
  (params (Instigator :type Pawn%20Object%20Reference) (Location :type Vector%20%28by%20ref%29 :default "0, 0, 0") (Volume :type Float%20%28single-precision%29))
  (bind _returnvalue (Utilities|Name|MakeLiteralName "hearedNoise?"))
  (bind _self self)
  (bind _returnvalue_2 (AI|GetAIController _self))
  (bind _returnvalue_3 (AI|GetBlackboard _returnvalue_2))
  (if true
    (AI|Components|Blackboard|SetValueasBool _returnvalue_3 _returnvalue true)
    (Utilities|FlowControl|Delay 1.0)
    (AI|Components|Blackboard|SetValueasBool _returnvalue_3 _returnvalue false)))

(event Custom|AttackPlayer
  (bind _attacktracepoint (Variables|Default|GetAttackTracePoint))
  (bind _returnvalue (Transformation|GetWorldLocation _attacktracepoint))
  (if (not (Variables|Default|Getattacking))
    (Variables|Default|Setattacking true)
    (Animation|Montage|PlayMontage (Variables|Character|GetMesh) "/Game/Enemy/GhostGirl/AnimationGirl/Zombie_Headbutt__2__Montage.Zombie_Headbutt__2__Montage"
      (:then
        (bind (_outhit _returnvalue_2) (Collision|SphereTraceForObjects _returnvalue (+ _returnvalue (* (Math|Vector|GetForwardVector (Transformation|GetWorldRotation _attacktracepoint)) 7e+01)) 25.0 (Utilities|Array|MakeArray "ObjectTypeQuery3") false 0 "None"))
        (if _returnvalue_2
          (Game|Damage|ApplyDamage (.HitActor (Collision|BreakHitResult _outhit)) 1e+01 0 0)
          (Audio|PlaySound2D "/Game/Audio/Jumpscare.Jumpscare" 1.0 1.0 0.0 0 0)))
      (:OnCompleted
        (Variables|Default|Setattacking false)))))

(event Custom|Stop%20seeing%20player
  (AI|Components|Blackboard|SetValueasBool (AI|GetBlackboard (AI|GetAIController self)) (Utilities|Name|MakeLiteralName "seeingPlayer") false))

(event EventBeginPlay
  (Utilities|FlowControl|Sequence
    (:then_0
      (Utilities|Time|SetTimerbyEvent (delegate Custom|Stop%20seeing%20player) 5.0 true))
    (:then_1
      (bind _returnvalue (AddComponent|AddAudioComponent false))
      (Audio|Components|Audio|Stop _returnvalue)
      (Variables|Default|SetChaseMusic _returnvalue))))

(event EventTick
  (params (DeltaSeconds :type Float%20%28single-precision%29))
  (if (not (Variables|Default|GetSee%20Enemy))
    (Utilities|FlowControl|Delay 0.4)
    (if (not (Variables|Default|GetSee%20Enemy))
      (Audio|Components|Audio|FadeOut (Variables|Default|GetChaseMusic) 3.0 0.0 "Linear" :!class /Script/Engine.AudioComponent)
      (Utilities|FlowControl|DoOnce false) ; enters at Reset
    )))

(fn ConstructionScript)