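; Secret bookshelf door Blueprint that swings a bookshelf open and closed when its Open/CloseDoor event fires.
; The event plays a door squeak, then a DoOnce gate feeds a FlipFlop, resetting when each timeline finishes.
; Opening lerps the special book's pitch and shelf's yaw on OpenTrack; closing reverses a separate DoorClose timeline that rotates only the shelf.
; The squeak precedes the gate, so it also plays on blocked calls.
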(event Custom|Open/Close%20Door
  (Audio|PlaySoundatLocation "/Game/Audio/346211__inspectorj__door-squeak-normal-e.346211__inspectorj__door-squeak-normal-e" (Transformation|GetActorLocation) "0, 0, 0" 1.0 1.0 0.0 0 0 0 0)
  (Utilities|FlowControl|DoOnce false :!label _label
    (:Completed
      (Utilities|FlowControl|FlipFlop
        (:A
          (bind (_direction _booktrack _doortrack) (Timeline|OpenTrack PlayFromStart)
            (:Update
              (Transformation|SetRelativeRotation (Variables|Default|GetSpecialBook) (Math|Rotator|MakeRotator 0.0 (Math|Float|Lerp (Variables|Default|GetBookIn) (Variables|Default|GetBookOut) _booktrack) -9e+01) false false)
              (Transformation|SetRelativeRotation (Variables|Default|GetBookshelf) (Math|Rotator|MakeRotator 0.0 0.0 (Math|Float|Lerp (Variables|Default|GetDoorClosed) (Variables|Default|GetDoorOpen) _doortrack)) false false))
            (:Finished
              (goto _label Reset))))
        (:B
          (bind _doortrack_2 (Timeline|DoorClose ReverseFromEnd)
            (:Update
              (Transformation|SetRelativeRotation (Variables|Default|GetBookshelf) (Math|Rotator|MakeRotator 0.0 0.0 (Math|Float|Lerp (Variables|Default|GetDoorClosed) (Variables|Default|GetDoorOpen) _doortrack_2)) false false))
            (:Finished
              (goto _label Reset))))))))

(fn ConstructionScript)