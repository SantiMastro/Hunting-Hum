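; BP_Hide is an interactable hiding spot that the player can enter and leave.
; Its Interact event toggles an Inside flag and teleports player character 0 to the RefInside or RefOutside reference transform.
; Each toggle also snaps the Door closed or open by setting its relative rotation and plays the matching door sound at the world origin.
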(event EventBeginPlay)

(event Collision|EventActorBeginOverlap
  (params (OtherActor :type Actor%20Object%20Reference)))

(event EventTick
  (params (DeltaSeconds :type Float%20%28single-precision%29)))

(event EventInteract
  (bind _refinside (Variables|Default|GetRefInside))
  (bind _refoutside (Variables|Default|GetRefOutside))
  (bind _returnvalue (Transformation|GetWorldTransform _refinside))
  (bind _returnvalue_2 (Transformation|GetWorldTransform _refoutside))
  (if (not (Variables|Default|GetInside?))
    (Variables|Default|SetInside? true)
    (Transformation|SetActorTransform (Game|GetPlayerCharacter 0) (Math|Transform|MakeTransform (.location _returnvalue) (.rotation _returnvalue) "1.000000,1.000000,1.000000"))
    (Audio|PlaySoundatLocation "/Game/Audio/364920__matrixxx__door-closing.364920__matrixxx__door-closing" "0, 0, 0" "0, 0, 0" 1.0 1.0 0.0 0 0 0 0)
    (Transformation|SetRelativeRotation (Variables|Default|GetDoor) "0, 0, 0" false false)
    (else
      (Variables|Default|SetInside? false)
      (Transformation|SetActorTransform (Game|GetPlayerCharacter 0) (Math|Transform|MakeTransform (.location _returnvalue_2) (.rotation _returnvalue_2) "1.000000,1.000000,1.000000"))
      (Audio|PlaySoundatLocation "/Game/Audio/704609__matrixxx__front-door-opening__mp3cut_net_.704609__matrixxx__front-door-opening__mp3cut_net_" "0, 0, 0" "0, 0, 0" 1.0 1.0 0.0 0 0 0 0)
      (Transformation|SetRelativeRotation (Variables|Default|GetDoor) "0.000000,100.000000,0.000000" false false))))

(fn ConstructionScript)