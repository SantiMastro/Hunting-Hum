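; BP_Door_2 is an interactable door that swings open and closed with a squeak sound.
; Interact alternates through a FlipFlop between playing and reversing DoorTimeline, whose track lerps the mesh's relative yaw from zero to the Rotation variable.
; The branch condition is fixed to true, so the else path's unlock sound never plays.
; PickUpKey sets HasKey to false, but Interact never reads it, so no key is required.
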(event EventInteract
  (if true
    (Audio|PlaySoundatLocation "/Game/Audio/346211__inspectorj__door-squeak-normal-e.346211__inspectorj__door-squeak-normal-e" (Transformation|GetActorLocation) "0, 0, 0" 1.0 1.0 0.0 0 0 0 0)
    (Utilities|FlowControl|FlipFlop
      (:A
        (bind _door_track (Timeline|Door%20Timeline Play)
          (:Update
            (Transformation|SetRelativeRotation (Variables|Default|GetStaticMesh) (Math|Rotator|MakeRotator 0.0 0.0 (Math|Float|Lerp 0.0 (Variables|Default|GetRotation) _door_track)) false false))))
      (:B
        (Timeline|Door%20Timeline Reverse)))
    (else
      (Audio|PlaySoundatLocation "/Game/Audio/519065__angelkunev__door-unlock.519065__angelkunev__door-unlock" (Transformation|GetActorLocation) "0, 0, 0" 1.0 1.0 0.0 0 0 0 0))))

(event EventPickUpKey
  (Variables|Default|SetHas%20Key? false))

(fn ConstructionScript)